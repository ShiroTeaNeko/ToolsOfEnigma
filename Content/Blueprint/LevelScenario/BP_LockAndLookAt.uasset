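; Scripted one-shot level trigger that pulls the first-person player's view toward a LookAt point with a zoom and sound cue.
; The first overlap of the Box by the player plays a boat horn at LookAt and fleeing birds at the player.
; A Timeline then overrides control rotation toward LookAt while easing FOV to half.
; A second Timeline eases FOV back to its saved value, using per-frame interpolation.
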(event `self.Box.OnComponentBeginOverlap`
  (params (OverlappedComponent :type "PrimitiveComponent Object Reference") (OtherActor :type "Actor Object Reference") (OtherComp :type "PrimitiveComponent Object Reference") (OtherBodyIndex :type Integer) (bFromSweep :type Boolean) (SweepResult :type "HitResult Structure (by ref)"))
  (bind _returnvalue (`GameplayStatics.GetWorldDeltaSeconds`))
  (bind _returnvalue_2 (`SceneComponent.K2_GetComponentLocation` (`self.LookAt`)))
  (`/Engine/EditorBlueprintResources/StandardMacros.IsValid` OtherActor
    (:`Is Valid`
      (bind _asbp_first_person_character (cast `/Game/FirstPerson/Blueprints/BP_FirstPersonCharacter` OtherActor))
      (`/Engine/EditorBlueprintResources/StandardMacros.DoOnce` false
        (:`Completed`
          (bind _firstpersoncamera (`/Game/FirstPerson/Blueprints/BP_FirstPersonCharacter.FirstPersonCamera` _asbp_first_person_character))
          (bind _fieldofview (`CameraComponent.FieldOfView` _firstpersoncamera))
          (set `self.FOV` _fieldofview)
          (`GameplayStatics.PlaySoundAtLocation` "/Game/Blueprint/LevelScenario/BoatHornSFX.BoatHornSFX" _returnvalue_2 (struct) 0.1 1.0 0.0 null null null null)
          (bind _returnvalue_3 (`self.K2_GetActorLocation` _asbp_first_person_character))
          (`GameplayStatics.PlaySoundAtLocation` "/Game/Blueprint/LevelScenario/BirdsFlyAway.BirdsFlyAway" _returnvalue_3 (struct) 0.3 1.0 0.0 null null null null)
          (`Timeline|Timeline`
            (:`Update`
              (`Controller.SetControlRotation` (`GameplayStatics.GetPlayerController` 0) (`KismetMathLibrary.RInterpTo` (`self.K2_GetActorRotation` _asbp_first_person_character) (`KismetMathLibrary.FindLookAtRotation` _returnvalue_3 _returnvalue_2) _returnvalue 2.0))
              (`CameraComponent.SetFieldOfView` _firstpersoncamera (`KismetMathLibrary.FInterpTo` _fieldofview (/ (`self.FOV`) 2.0) _returnvalue 2.0)))
            (:`Finished`
              (`Timeline|Timeline_0`
                (:`Update`
                  (`CameraComponent.SetFieldOfView` _firstpersoncamera (`KismetMathLibrary.FInterpTo` _fieldofview (`self.FOV`) (`GameplayStatics.GetWorldDeltaSeconds`) 2.0)))))))))))

(fn `UserConstructionScript`)