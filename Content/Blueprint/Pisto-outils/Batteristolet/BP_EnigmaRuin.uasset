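; BP_EnigmaRuin is a ruin puzzle that completes once its four batteries, BatA through BatD, are all charged.
; On BeginPlay it binds to each battery's charged event and gathers them in AllBat.
; Each charge event runs CheckAllBat, which scans the array for any uncharged battery.
; On success it zeroes the Portal's AmountToFinish, plays the achievement sound and triggers the portal's enigma finish message.
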(event `self.ReceiveBeginPlay`
  (bind _bat_a (`self.Bat A`))
  (bind _bat_d (`self.Bat D`))
  (bind _bat_c (`self.Bat C`))
  (bind _bat_b (`self.Bat B`))
  (`parent.ReceiveBeginPlay`)
  (add `/Game/Blueprint/Pisto-outils/Batteristolet/Battery.BatteryCharged` _bat_a (delegate `CallBatA`))
  (`KismetArrayLibrary.Array_Add` (`self.AllBat`) _bat_a)
  (add `/Game/Blueprint/Pisto-outils/Batteristolet/Battery.BatteryCharged` _bat_b (delegate `CallBatB`))
  (`KismetArrayLibrary.Array_Add` (`self.AllBat`) _bat_b)
  (add `/Game/Blueprint/Pisto-outils/Batteristolet/Battery.BatteryCharged` _bat_c (delegate `CallBatC`))
  (`KismetArrayLibrary.Array_Add` (`self.AllBat`) _bat_c)
  (add `/Game/Blueprint/Pisto-outils/Batteristolet/Battery.BatteryCharged` _bat_d (delegate `CallBatD`))
  (`KismetArrayLibrary.Array_Add` (`self.AllBat`) _bat_d))

(event `CallBatA`
  (bind _portal (`self.Portal`))
  (`self.CheckAllBat` :!label _label)
  (if (`self.isDone`)
    (set `/Game/Alexis/BP/BP_DoorDropPipe.AmountToFinish` 0 _portal)
    (`GameplayStatics.PlaySound2D` "/Game/Sound/Achievement-Sound-Effect.Achievement-Sound-Effect" 1.0 1.0 0.0 null null)
    (message `/Game/Alexis/BP/I_Enigma.EnigmaFinish` _portal)))

(event `CallBatC`
  (goto _label))

(event `CallBatD`
  (goto _label))

(event `CallBatB`
  (goto _label))

(fn `CheckAllBat`
  (set `self.isDone` true)
  (for _array_element (`self.AllBat`)
    (if (not (`/Game/Blueprint/Pisto-outils/Batteristolet/Battery.isCharged` _array_element))
      (set `self.isDone` false)
      (break)))
  (return))

(fn `UserConstructionScript`
  (`parent.UserConstructionScript`))