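; Moving platform that travels between a Start and an End point, optionally held until a linked enigma is done.
; The construction script adds both points as relative control points on an InterpToMovement component.
; When EnigmaDone is valid, BeginPlay disables that component's tick and binds Move to the done event, which re-enables it.
; Without a valid EnigmaDone, the component's tick is left untouched.
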(event `self.ReceiveBeginPlay`
  (bind _enigmadone (`self.EnigmaDone`))
  (`/Engine/EditorBlueprintResources/StandardMacros.IsValid` _enigmadone
    (:`Is Valid`
      (add `/Game/Blueprint/Pisto-outils/Batteristolet/BP_EnigmaDone.Done` _enigmadone (delegate `Move`))
      (`ActorComponent.SetComponentTickEnabled` (`self.InterpToMovement`) false))))

(event `Move`
  (`ActorComponent.SetComponentTickEnabled` (`self.InterpToMovement`) true))

(fn `UserConstructionScript`
  (`InterpToMovementComponent.AddControlPointPosition` (`self.InterpToMovement`) (`self.Start`) true)
  (`InterpToMovementComponent.AddControlPointPosition` (`self.InterpToMovement`) (`self.End`) true))