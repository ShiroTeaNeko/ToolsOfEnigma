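; BP_EnigmaMultiBattery is a child puzzle Blueprint with four batteries in a Lights Out style chain, solved when all are charged.
; On BeginPlay it binds each battery's charged event and stores the batteries in an array.
; Each event toggles the adjacent batteries (A-B-C-D, no wraparound) through SwapBattery, which also recomputes IsDone across the array.
; The new state feeds ChargeBattery, then CheckDone defers to the parent class.
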(event `self.ReceiveBeginPlay`
  (bind _batteryb (`self.batteryB`))
  (bind _batteryd (`self.batteryD`))
  (bind _batterya (`self.batteryA`))
  (bind _batteryc (`self.batteryC`))
  (add `/Game/Blueprint/Pisto-outils/Batteristolet/Battery.BatteryCharged` _batterya (delegate `CallBatteryA`))
  (`KismetArrayLibrary.Array_Add` (`self.AllBatteries`) _batterya)
  (add `/Game/Blueprint/Pisto-outils/Batteristolet/Battery.BatteryCharged` _batteryb (delegate `CallBatteryB`))
  (`KismetArrayLibrary.Array_Add` (`self.AllBatteries`) _batteryb)
  (add `/Game/Blueprint/Pisto-outils/Batteristolet/Battery.BatteryCharged` _batteryc (delegate `CallBatteryC`))
  (`KismetArrayLibrary.Array_Add` (`self.AllBatteries`) _batteryc)
  (add `/Game/Blueprint/Pisto-outils/Batteristolet/Battery.BatteryCharged` _batteryd (delegate `CallBatteryD`))
  (`KismetArrayLibrary.Array_Add` (`self.AllBatteries`) _batteryd))

(event `CallBatteryA`
  (bind _batteryb (`self.batteryB`))
  (bind _ischarged (`self.SwapBattery` _batteryb))
  (`/Game/Blueprint/Pisto-outils/Batteristolet/Battery.ChargeBattery` _batteryb _ischarged)
  (`self.CheckDone`))

(event `CallBatteryB`
  (bind _batteryc (`self.batteryC`))
  (bind _batterya (`self.batteryA`))
  (`|ExecutionSequence`
    (:`then_0`
      (bind _ischarged (`self.SwapBattery` _batterya))
      (`/Game/Blueprint/Pisto-outils/Batteristolet/Battery.ChargeBattery` _batterya _ischarged))
    (:`then_1`
      (bind _ischarged_2 (`self.SwapBattery` _batteryc))
      (`/Game/Blueprint/Pisto-outils/Batteristolet/Battery.ChargeBattery` _batteryc _ischarged_2)
      (`self.CheckDone`))))

(event `CallBatteryC`
  (bind _batteryb (`self.batteryB`))
  (bind _batteryd (`self.batteryD`))
  (`|ExecutionSequence`
    (:`then_0`
      (bind _ischarged (`self.SwapBattery` _batteryb))
      (`/Game/Blueprint/Pisto-outils/Batteristolet/Battery.ChargeBattery` _batteryb _ischarged))
    (:`then_1`
      (bind _ischarged_2 (`self.SwapBattery` _batteryd))
      (`/Game/Blueprint/Pisto-outils/Batteristolet/Battery.ChargeBattery` _batteryd _ischarged_2)
      (`self.CheckDone`))))

(event `CallBatteryD`
  (bind _batteryc (`self.batteryC`))
  (bind _ischarged (`self.SwapBattery` _batteryc))
  (`/Game/Blueprint/Pisto-outils/Batteristolet/Battery.ChargeBattery` _batteryc _ischarged)
  (`self.CheckDone`))

(fn `CheckDone`
  (`parent.CheckDone`))

(fn `SwapBattery`
  (params (Battery :type "/Game/Blueprint/Pisto-outils/Batteristolet/Battery Object Reference"))
  (returns (isCharged :type Boolean))
  (bind _output_get (set `/Game/Blueprint/Pisto-outils/Batteristolet/Battery.isCharged` (not (`/Game/Blueprint/Pisto-outils/Batteristolet/Battery.isCharged` Battery)) Battery))
  (set `self.isDone` true)
  (for _array_element (`self.AllBatteries`)
    (if (not (`/Game/Blueprint/Pisto-outils/Batteristolet/Battery.isCharged` _array_element))
      (set `self.isDone` false)
      (break)))
  (return _output_get))

(fn `UserConstructionScript`
  (`parent.UserConstructionScript`))