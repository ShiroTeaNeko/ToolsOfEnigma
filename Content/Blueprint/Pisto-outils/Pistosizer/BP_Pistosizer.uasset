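; Pistosizer gun, a gatherable pickup that shrinks or grows either the player character or physics objects, depending on its mode.
; Gather adds it to the player's inventory, equips it, shows weapon UI and destroys the pickup.
; While visible, the two fire events step the target's index through preset scales.
; Object mode line-traces from the camera for simulating BP_BaseActorScalable actors, scaling their size from a base and multiplying their mass.
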(event `self.ReceiveBeginPlay`
  (bind _owningcharacter (`self.OwningCharacter`))
  (bind _asbp_first_person_character (cast `/Game/FirstPerson/Blueprints/BP_FirstPersonCharacter` (`GameplayStatics.GetPlayerCharacter` 0)))
  (set `self.OwningCharacter` _asbp_first_person_character)
  (add `/Game/FirstPerson/Blueprints/BP_FirstPersonCharacter.GunFire` _owningcharacter (delegate `Fire`))
  (add `/Game/FirstPerson/Blueprints/BP_FirstPersonCharacter.GunFire2` _owningcharacter (delegate `Fire2`))
  (add `self.RunTimeline` (delegate `CallTimeline`))
  (if (not (`self.isGatherable`))
    (`PrimitiveComponent.SetCollisionEnabled` (`self.Sphere`) "NoCollision")))

(event `Fire`
  (if (`SceneComponent.bVisible` (`/Game/FirstPerson/Blueprints/BP_FirstPersonCharacter.BP_Pistosizer` (`self.OwningCharacter`)))
    (`self.AttemptScale` 1 2.0)))

(event `Fire2`
  (if (`SceneComponent.bVisible` (`/Game/FirstPerson/Blueprints/BP_FirstPersonCharacter.BP_Pistosizer` (`self.OwningCharacter`)))
    (`self.AttemptScale` -1 0.5)))

(event `CallTimeline`
  (bind (_direction _newtrack_0) (`Timeline|ScaleObject` :!via `PlayFromStart`)
    (:`Update`
      (set `self.TimeLineFloat` _newtrack_0))))

(event `/Game/FirstPerson/Blueprints/I_Gatherable.Gather`
  (bind _asbp_first_person_character (cast `/Game/FirstPerson/Blueprints/BP_FirstPersonCharacter` (`GameplayStatics.GetPlayerCharacter` 0)))
  (set `/Game/FirstPerson/Blueprints/BP_FirstPersonCharacter.CurrentlyEquippedWeapon` 2 _asbp_first_person_character)
  (`/Game/FirstPerson/Blueprints/BP_FirstPersonCharacter.AddPistoToInventory` _asbp_first_person_character (`/Game/FirstPerson/Blueprints/BP_FirstPersonCharacter.BP_Pistosizer` _asbp_first_person_character))
  (`/Game/FirstPerson/Blueprints/BP_FirstPersonCharacter.EquipPisto` _asbp_first_person_character (`/Game/FirstPerson/Blueprints/BP_FirstPersonCharacter.GunInventory` _asbp_first_person_character))
  (bind _ashud_first_person_character (cast `/Game/FirstPerson/Blueprints/HUD_FirstPersonCharacter` (`/Game/FirstPerson/Blueprints/BP_FirstPersonCharacter.HUD` _asbp_first_person_character)))
  (`/Game/FirstPerson/Blueprints/HUD_FirstPersonCharacter.ShowUIWeaponEvent` _ashud_first_person_character)
  (`self.K2_DestroyActor`))

(fn `AttemptScale`
  (params (ScaleDirection :type Integer) (ScaleMult :type "Float (double-precision)"))
  (bind _owningcharacter (`self.OwningCharacter`))
  (bind _scales (`self.Scales`))
  (bind _returnvalue (+ ScaleDirection (`/Game/FirstPerson/Blueprints/BP_FirstPersonCharacter.CurrentScaleMult` _owningcharacter)))
  (switch `/Game/Blueprint/Pisto-outils/Pistosizer/E_PistosizerMode` (`self.PistosizerMode`)
    (:`NewEnumerator0`
      (set `self.ActorToScale` _owningcharacter)
      (if (`KismetArrayLibrary.Array_IsValidIndex` _scales _returnvalue)
        (bind _output_get (set `/Game/FirstPerson/Blueprints/BP_FirstPersonCharacter.CurrentScaleMult` _returnvalue _owningcharacter))
        (`self.SetScale` (`self.Scales`) _output_get)
        (elif (< _returnvalue 0)
          (bind _output_get_2 (set `/Game/FirstPerson/Blueprints/BP_FirstPersonCharacter.CurrentScaleMult` 0 _owningcharacter))
          (`self.SetScale` (`self.Scales`) _output_get_2)
          (else
            (bind _output_get_3 (set `/Game/FirstPerson/Blueprints/BP_FirstPersonCharacter.CurrentScaleMult` 2 _owningcharacter))
            (`self.SetScale` (`self.Scales`) _output_get_3)))))
    (:`NewEnumerator1`
      (`self.LineTraceObject`)
      (bind _asbp_base_actor_scalable (cast `/Game/Blueprint/Pisto-outils/Pistosizer/BP_BaseActorScalable` (`self.ActorToScale`)))
      (set `self.ActorBaseScale` (`/Game/Blueprint/Pisto-outils/Pistosizer/BP_BaseActorScalable.BaseScale` _asbp_base_actor_scalable))
      (bind _returnvalue_2 (+ ScaleDirection (`/Game/Blueprint/Pisto-outils/Pistosizer/BP_BaseActorScalable.CurrentScaleMult` _asbp_base_actor_scalable)))
      (if (`KismetArrayLibrary.Array_IsValidIndex` _scales _returnvalue_2)
        (bind _output_get_4 (set `/Game/Blueprint/Pisto-outils/Pistosizer/BP_BaseActorScalable.CurrentScaleMult` _returnvalue_2 _asbp_base_actor_scalable))
        (`self.SetScale` (`self.Scales`) _output_get_4 ScaleMult)
        (elif (< _returnvalue_2 0)
          (set `/Game/Blueprint/Pisto-outils/Pistosizer/BP_BaseActorScalable.CurrentScaleMult` 0 _asbp_base_actor_scalable)
          (else
            (set `/Game/Blueprint/Pisto-outils/Pistosizer/BP_BaseActorScalable.CurrentScaleMult` 2 _asbp_base_actor_scalable)))))))

(fn `LineTraceObject`
  (bind _firstpersoncamera (`/Game/FirstPerson/Blueprints/BP_FirstPersonCharacter.FirstPersonCamera` (`self.OwningCharacter`)))
  (bind _returnvalue (`SceneComponent.K2_GetComponentLocation` _firstpersoncamera))
  (bind (_outhit _returnvalue_2) (`KismetSystemLibrary.LineTraceSingle` :`Start` _returnvalue :`End` (+ _returnvalue (* (`KismetMathLibrary.GetForwardVector` (`SceneComponent.K2_GetComponentRotation` _firstpersoncamera)) 2000.0)) :`TraceChannel` "TraceTypeQuery1" :`DrawDebugType` "ForDuration" :`DrawTime` 1.5))
  (if _returnvalue_2
    (bind (_bblockinghit _binitialoverlap _time _distance _location _impactpoint _normal _impactnormal _physmat _hitactor) (`GameplayStatics.BreakHitResult` _outhit))
    (bind _returnvalue_3 (`SceneComponent.IsAnySimulatingPhysics` (`Actor.RootComponent` _hitactor)))
    (if _returnvalue_3
      (set `self.Is Object Hit` _returnvalue_3)
      (set `self.ActorToScale` _hitactor)
      (else
        (set `self.Is Object Hit` false)))))

(fn `SetScale`
  (params (Scales :type "Array of Vector Structure") (current :type Integer) (ScaleMult :type "Float (double-precision)"))
  (`self.SetActorScale3D` (`self.ActorToScale`) (* (`self.ActorBaseScale`) (`|GetArrayItem` Scales current)))
  (bind _asbp_base_actor_scalable (cast `/Game/Blueprint/Pisto-outils/Pistosizer/BP_BaseActorScalable` (`self.ActorToScale`)))
  (bind _box (`/Game/Blueprint/Pisto-outils/Pistosizer/BP_BaseActorScalable.Box` _asbp_base_actor_scalable))
  (bind _returnvalue (`PrimitiveComponent.GetMass` _box))
  (`KismetSystemLibrary.PrintString` (`KismetStringLibrary.Conv_DoubleToString` _returnvalue))
  (`PrimitiveComponent.SetMassOverrideInKg` _box "None" (* _returnvalue ScaleMult) true)
  (set `self.ActorToScale` null))

(fn `UserConstructionScript`)