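; BP_BaseActorScalable is a base actor for scalable objects, filed under the Pistosizer tool.
; Its construction script calls SetMesh to apply the NewUsedMesh variable to the static mesh component.
; On BeginPlay it records the mesh's mass as CurrentWeight and the Box component's world scale as BaseScale.
; The scaling logic itself is not in this Blueprint.
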(event `self.ReceiveBeginPlay`
  (set `self.currentWeight` (`PrimitiveComponent.GetMass` (`self.StaticMesh`)))
  (set `self.BaseScale` (`SceneComponent.K2_GetComponentScale` (`self.Box`))))

(fn `SetMesh`
  (`StaticMeshComponent.SetStaticMesh` (`self.StaticMesh`) (`self.NewUsedMesh`)))

(fn `UserConstructionScript`
  (`self.SetMesh`))