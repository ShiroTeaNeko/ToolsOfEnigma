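; Grappling-hook gun (Attrapistolet) that can be gathered as a pickup, then pulls physics objects to the player or the player to grapple targets.
; Firing line-traces from the camera and spawns a hook and cable line toward a physics object or the current target.
; Tick-driven state machines either lob the object with a suggested-arc impulse or hop and fly the player, with a stuck timeout.
; While retracted, it highlights the visible target nearest the view direction.
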(event `self.DetectCollision.OnComponentBeginOverlap`
  (params (OverlappedComponent :type "PrimitiveComponent Object Reference") (OtherActor :type "Actor Object Reference") (OtherComp :type "PrimitiveComponent Object Reference") (OtherBodyIndex :type Integer) (bFromSweep :type Boolean) (SweepResult :type "HitResult Structure (by ref)"))
  (if (not (`self.IsPistoEquipped`))
    (cast `/Game/FirstPerson/Blueprints/BP_FirstPersonCharacter` OtherActor)
    (`/Engine/EditorBlueprintResources/StandardMacros.IsValid` (`self.UIInteract`)
      (:`Is Not Valid`
        (bind _returnvalue (`|CreateWidget` "/Game/Alexis/UI/UIInteract.UIInteract_C"))
        (bind _output_get (set `self.UIInteract` _returnvalue))
        (`UserWidget.AddToViewport` _returnvalue 0)
        (`UserWidget.AddToViewport` _output_get 0)))))

(event `self.ReceiveBeginPlay`
  (bind _asbp_first_person_character (cast `/Game/FirstPerson/Blueprints/BP_FirstPersonCharacter` (`GameplayStatics.GetPlayerCharacter` 0)))
  (set `self.OwningCharacter` _asbp_first_person_character)
  (add `/Game/FirstPerson/Blueprints/BP_FirstPersonCharacter.GunFire` (`self.OwningCharacter`) (delegate `Fire`))
  (if (not (`self.isGatherable`))
    (`PrimitiveComponent.SetCollisionEnabled` (`self.Sphere`) "NoCollision")))

(event `self.DetectCollision.OnComponentEndOverlap`
  (params (OverlappedComponent :type "PrimitiveComponent Object Reference") (OtherActor :type "Actor Object Reference") (OtherComp :type "PrimitiveComponent Object Reference") (OtherBodyIndex :type Integer))
  (cast `/Game/FirstPerson/Blueprints/BP_FirstPersonCharacter` OtherActor)
  (`/Engine/EditorBlueprintResources/StandardMacros.IsValid` (`self.UIInteract`) :!label _label
    (:`Is Valid`
      (`Widget.RemoveFromParent` (`self.UIInteract`))
      (set `self.UIInteract` null))))

(event `Fire`
  (if (`SceneComponent.bVisible` (`/Game/FirstPerson/Blueprints/BP_FirstPersonCharacter.BP_Attrapistolet` (`self.OwningCharacter`)))
    (`self.Line Trace Detect Object`)
    (if (`self.IsObjectHit`)
      (`self.AttemptGrappleObject`)
      (else
        (`self.AttemptGrappleSurface`)
        (set `self.TimeToSwapIfStuck` 0.0)))
    (`GameplayStatics.PlaySoundAtLocation` "/Game/Blueprint/Pisto-outils/Attrapistolet/GrappleStart.GrappleStart" (`self.K2_GetActorLocation`) (struct) 1.0 1.0 0.0 null null null null)))

(event `RemoveInteract`
  (goto _label))

(event `self.ReceiveTick`
  (params (DeltaSeconds :type "Float (single-precision)"))
  (if (`self.IsObjectHit`)
    (switch `/Game/Blueprint/Pisto-outils/Attrapistolet/EAttrapistoletObjectState` (`self.GrappleObjectState`)
      (:`NewEnumerator2`
        (`self.TickVelocityLaunch`))
      (:`NewEnumerator4`
        (`KismetSystemLibrary.Delay` 0.5)
        (set `self.GrappleObjectState` "NewEnumerator3"))
      (:`NewEnumerator3`
        (`self.TickOnTargetObject`)))
    (elif (`SceneComponent.bVisible` (`/Game/FirstPerson/Blueprints/BP_FirstPersonCharacter.BP_Attrapistolet` (`self.OwningCharacter`)))
      (switch `/Game/Blueprint/Pisto-outils/Attrapistolet/EAttrapistoletState` (`self.GrappleState`)
        (:`NewEnumerator0`
          (`self.TickRetracted`))
        (:`NewEnumerator1`
          (`self.TickFiring`)
          (goto _label_2 :!via `Reset`))
        (:`NewEnumerator2`
          (`self.TickNearingTarget`))
        (:`NewEnumerator3`
          (`self.TickOnTarget`)))
      (else
        (bind _currenttarget (`self.CurrentTarget`)
          (:`then`
            (`/Game/Blueprint/Pisto-outils/Attrapistolet/BP_AttrapistoletTarget.SetActive` _currenttarget false)
            (set `self.GrappleState` "NewEnumerator0")
            (`self.GrappleLine`
              (:`then`
                (`self.GrappleHook`
                  (:`then`
                    (`/Engine/EditorBlueprintResources/StandardMacros.DoOnce` false :!label _label_2
                      (:`Completed`
                        (`self.RemoveGrapple`))))
                  (:`else`)))
              (:`else`)))
          (:`else`))))))

(event `/Game/FirstPerson/Blueprints/I_Gatherable.Gather`
  (bind _asbp_first_person_character (cast `/Game/FirstPerson/Blueprints/BP_FirstPersonCharacter` (`GameplayStatics.GetPlayerCharacter` 0)))
  (set `/Game/FirstPerson/Blueprints/BP_FirstPersonCharacter.CurrentlyEquippedWeapon` 0 _asbp_first_person_character)
  (`/Game/FirstPerson/Blueprints/BP_FirstPersonCharacter.AddPistoToInventory` _asbp_first_person_character (`/Game/FirstPerson/Blueprints/BP_FirstPersonCharacter.BP_Attrapistolet` _asbp_first_person_character))
  (`/Game/FirstPerson/Blueprints/BP_FirstPersonCharacter.EquipPisto` _asbp_first_person_character (`/Game/FirstPerson/Blueprints/BP_FirstPersonCharacter.GunInventory` _asbp_first_person_character))
  (bind _ashud_first_person_character (cast `/Game/FirstPerson/Blueprints/HUD_FirstPersonCharacter` (`/Game/FirstPerson/Blueprints/BP_FirstPersonCharacter.HUD` _asbp_first_person_character)))
  (`/Game/FirstPerson/Blueprints/HUD_FirstPersonCharacter.ShowUIWeaponEvent` _ashud_first_person_character)
  (set `/Game/FirstPerson/Blueprints/HUD_FirstPersonCharacter.LastEquippedWeapon` 0 _ashud_first_person_character)
  (`self.K2_DestroyActor`)
  (`self.RemoveInteract`))

(fn `AttemptGrappleObject`
  (bind _arrow (`self.Arrow`))
  (bind _returnvalue (`SceneComponent.K2_GetComponentLocation` _arrow))
  (switch `/Game/Blueprint/Pisto-outils/Attrapistolet/EAttrapistoletObjectState` (`self.GrappleObjectState`)
    (:`NewEnumerator0`
      (bind _grappleobjecttarget (`self.GrappleObjectTarget`)
        (:`then`
          (bind _returnvalue_2 (`|SpawnActorFromClass` "/Game/Blueprint/Pisto-outils/Attrapistolet/BP_AttrapistoletHook.BP_AttrapistoletHook_C" (`KismetMathLibrary.MakeTransform` _returnvalue) "Undefined" "OverrideRootScale" null null 2500.0 _grappleobjecttarget true null))
          (set `self.GrappleHook` _returnvalue_2)
          (bind _returnvalue_3 (`|SpawnActorFromClass` "/Game/Blueprint/Pisto-outils/Attrapistolet/BP_AttrapistoletLine.BP_AttrapistoletLine_C" (`KismetMathLibrary.MakeTransform` _returnvalue) "AlwaysSpawn" "OverrideRootScale" null null))
          (bind _output_get (set `self.GrappleLine` _returnvalue_3))
          (`self.K2_AttachToComponent` _output_get _arrow "None" "SnapToTarget" "SnapToTarget" "SnapToTarget" true)
          (`CableComponent.SetAttachEndTo` (`CableActor.CableComponent` (`self.GrappleLine`)) (`self.GrappleHook`) "DefaultSceneRoot" "None")
          (set `self.GrappleObjectState` "NewEnumerator2"))
        (:`else`)))))

(fn `AttemptGrappleSurface`
  (bind _arrow (`self.Arrow`))
  (bind _returnvalue (`SceneComponent.K2_GetComponentLocation` _arrow))
  (switch `/Game/Blueprint/Pisto-outils/Attrapistolet/EAttrapistoletState` (`self.GrappleState`)
    (:`NewEnumerator0`
      (bind _currenttarget (`self.CurrentTarget`)
        (:`then`
          (bind _returnvalue_2 (`|SpawnActorFromClass` "/Game/Blueprint/Pisto-outils/Attrapistolet/BP_AttrapistoletHook.BP_AttrapistoletHook_C" (`KismetMathLibrary.MakeTransform` _returnvalue) "Undefined" "OverrideRootScale" null _currenttarget 2500.0 null false null))
          (set `self.GrappleHook` _returnvalue_2)
          (bind _returnvalue_3 (`|SpawnActorFromClass` "/Game/Blueprint/Pisto-outils/Attrapistolet/BP_AttrapistoletLine.BP_AttrapistoletLine_C" (`KismetMathLibrary.MakeTransform` _returnvalue) "AlwaysSpawn" "OverrideRootScale" null null))
          (bind _output_get (set `self.GrappleLine` _returnvalue_3))
          (`self.K2_AttachToComponent` _output_get _arrow "None" "SnapToTarget" "SnapToTarget" "SnapToTarget" true)
          (`CableComponent.SetAttachEndTo` (`CableActor.CableComponent` (`self.GrappleLine`)) (`self.GrappleHook`) "DefaultSceneRoot" "None")
          (set `self.GrappleState` "NewEnumerator1"))
        (:`else`)))))

(fn `FindBestTarget`
  (params (Targets :type "Array of Actor Object Reference"))
  (returns (Target :type "Actor Object Reference"))
  (locals (`CurrentTarget (local)` :type "Actor Object Reference") (`CurrentAngle (local)` :type "Float (double-precision)" :default 0.0) (`BestAngle (local)` :type "Float (double-precision)") (`BestTarget (local)` :type "Actor Object Reference"))
  (bind _owningcharacter (`self.OwningCharacter`))
  (bind _owningcharacter_2 (`self.OwningCharacter`))
  (for _array_element Targets
    (set `local.CurrentTarget (local)` _array_element)
    (`/Engine/EditorBlueprintResources/StandardMacros.IsValid` _owningcharacter
      (:`Is Valid`
        (bind (_outhit _returnvalue) (`KismetSystemLibrary.LineTraceSingle` (`self.K2_GetActorLocation` _owningcharacter) (`self.K2_GetActorLocation` (`local.CurrentTarget (local)`)) "TraceTypeQuery1" false (`|MakeArray` (`self.OwningCharacter`) :!type "Actor Object Reference")))
        (if _returnvalue
          (if (== (`.HitActor` (`GameplayStatics.BreakHitResult` _outhit)) (`local.CurrentTarget (local)`))
            (`|ExecutionSequence`
              (:`then_0`
                ;[1 1 1] calculate angle to target
                (`/Engine/EditorBlueprintResources/StandardMacros.IsValid` _owningcharacter_2
                  (:`Is Valid`
                    (set `local.CurrentAngle (local)` (`KismetMathLibrary.DegAcos` (`KismetMathLibrary.Dot_VectorVector` (`KismetMathLibrary.Normal` (- (`self.K2_GetActorLocation` (`local.CurrentTarget (local)`)) (`self.K2_GetActorLocation` _owningcharacter_2))) (`SceneComponent.GetForwardVector` (`/Game/FirstPerson/Blueprints/BP_FirstPersonCharacter.FirstPersonCamera` _owningcharacter_2))))))))
              (:`then_1`
                ;[1 1 1] if angle less than current target, take this as new target
                (if (or (< (`local.CurrentAngle (local)`) (`local.BestAngle (local)`)) (not (`KismetSystemLibrary.IsValid` (`local.BestTarget (local)`))))
                  (set `local.BestTarget (local)` (`local.CurrentTarget (local)`))
                  (set `local.BestAngle (local)` (`local.CurrentAngle (local)`))))))))))
  (return (`local.BestTarget (local)`)))

(fn `Interact`
  (params (Player :type "/Game/FirstPerson/Blueprints/BP_FirstPersonCharacter Object Reference"))
  (returns (bIsSucess :type Boolean))
  (return false))

(fn `Line Trace Detect Object`
  (bind _firstpersoncamera (`/Game/FirstPerson/Blueprints/BP_FirstPersonCharacter.FirstPersonCamera` (`self.OwningCharacter`)))
  (bind _returnvalue (`SceneComponent.K2_GetComponentLocation` _firstpersoncamera))
  (bind (_outhit _returnvalue_2) (`KismetSystemLibrary.LineTraceSingle` :`Start` _returnvalue :`End` (+ _returnvalue (* (`KismetMathLibrary.GetForwardVector` (`SceneComponent.K2_GetComponentRotation` _firstpersoncamera)) 2000.0)) :`TraceChannel` "TraceTypeQuery1" :`DrawTime` 1.5))
  (if _returnvalue_2
    (bind (_bblockinghit _binitialoverlap _time _distance _location _impactpoint _normal _impactnormal _physmat _hitactor) (`GameplayStatics.BreakHitResult` _outhit))
    (bind _returnvalue_3 (`SceneComponent.IsAnySimulatingPhysics` (`Actor.RootComponent` _hitactor)))
    (if _returnvalue_3
      (set `self.IsObjectHit` _returnvalue_3)
      (set `self.GrappleObjectTarget` _hitactor)
      (else
        (set `self.IsObjectHit` false)))))

(fn `RemoveGrapple`
  (`self.K2_DestroyActor` (`self.GrappleLine`))
  (set `self.GrappleLine` null)
  (`self.K2_DestroyActor` (`self.GrappleHook`))
  (set `self.GrappleHook` null))

(fn `SetCurrentTarget`
  (params (NewTarget :type "/Game/Blueprint/Pisto-outils/Attrapistolet/BP_AttrapistoletTarget Object Reference"))
  (if (!= NewTarget (`self.CurrentTarget`))
    (`|ExecutionSequence`
      (:`then_0`
        (bind _currenttarget (`self.CurrentTarget`)
          (:`then`
            (`/Game/Blueprint/Pisto-outils/Attrapistolet/BP_AttrapistoletTarget.SetActive` _currenttarget false)
            (set `/Game/Blueprint/Pisto-outils/Attrapistolet/BP_AttrapistoletTarget.isActive` false _currenttarget))
          (:`else`)))
      (:`then_1`
        (set `self.CurrentTarget` (`local.NewTarget`)))
      (:`then_2`
        (bind _currenttarget_2 (`self.CurrentTarget`)
          (:`then`
            (`/Game/Blueprint/Pisto-outils/Attrapistolet/BP_AttrapistoletTarget.SetActive` _currenttarget_2 true)
            (set `/Game/Blueprint/Pisto-outils/Attrapistolet/BP_AttrapistoletTarget.isActive` true _currenttarget_2))
          (:`else`))))))

(fn `TickFiring`
  (bind _owningcharacter (`self.OwningCharacter`))
  (if (< (`/Game/Blueprint/Pisto-outils/Attrapistolet/BP_AttrapistoletHook.DistanceToTarget` (`self.GrappleHook`)) (`self.StartJumpDistance`))
    (`/Engine/EditorBlueprintResources/StandardMacros.IsValid` _owningcharacter
      (:`Is Valid`
        (`Character.LaunchCharacter` _owningcharacter (0.0 0.0 500.0) true true)
        (set `self.GrappleState` "NewEnumerator2")))))

(fn `TickGetObject`
  (params (Object :type "Actor Object Reference"))
  (set `self.GrappleObjectTarget` Object))

(fn `TickNearingTarget`
  (bind _owningcharacter (`self.OwningCharacter`))
  (bind (_returnvalue_x _returnvalue_y _returnvalue_z) (`KismetMathLibrary.BreakVector` (`self.GetVelocity` _owningcharacter)))
  (`/Engine/EditorBlueprintResources/StandardMacros.IsValid` _owningcharacter
    (:`Is Valid`
      (if (<= _returnvalue_z 0.0)
        (set `self.InitialDirection` (`self.OwnerToTarget`))
        (set `self.GrappleState` "NewEnumerator3")))))

(fn `TickObjectNearingPlayer`
  (bind _grappleobjecttarget (`self.GrappleObjectTarget`))
  (bind _owningcharacter (`self.OwningCharacter`))
  (`/Engine/EditorBlueprintResources/StandardMacros.IsValid` _grappleobjecttarget
    (:`Is Valid`
      (`/Engine/EditorBlueprintResources/StandardMacros.IsValid` _owningcharacter
        (:`Is Valid`
          (if (<= (`self.GetDistanceTo` _owningcharacter _grappleobjecttarget) 500.0)
            (set `self.GrappleObjectState` "NewEnumerator3")))))))

(fn `TickOnTarget`
  (bind _initialdirection (`self.InitialDirection`))
  (bind _owningcharacter (`self.OwningCharacter`))
  (bind (_returnvalue_x _returnvalue_y) (`KismetMathLibrary.BreakVector` (* _initialdirection 250.0)))
  (bind (_returnvalue_x_2 _returnvalue_y_2 _returnvalue_z) (`KismetMathLibrary.BreakVector` (* _initialdirection 1.0)))
  (if (< (`self.GetDistanceTo` (`self.OwningCharacter`) (`self.CurrentTarget`)) (`self.EndJumpDistance`))
    (`Character.LaunchCharacter` _owningcharacter (`KismetMathLibrary.MakeVector` _returnvalue_x _returnvalue_y (`KismetMathLibrary.FMax` _returnvalue_z 600.0)) true true)
    (`self.SetCurrentTarget` null)
    (`self.RemoveGrapple`)
    (set `self.GrappleState` "NewEnumerator0")
    (else
      (set `MovementComponent.Velocity` (* (`self.OwnerToTarget`) (`self.CharacterGrappleSpeed`)) (`Pawn.GetMovementComponent` _owningcharacter))
      (set `self.TimeToSwapIfStuck` (+ (`self.TimeToSwapIfStuck`) (`GameplayStatics.GetWorldDeltaSeconds`)))
      (if (>= (`self.TimeToSwapIfStuck`) (`self.MaxTimeToSwapIfStuck`))
        (`self.SetCurrentTarget` null)
        (`self.RemoveGrapple`)
        (set `self.GrappleState` "NewEnumerator0")))))

(fn `TickOnTargetObject`
  (`self.RemoveGrapple`)
  (set `self.IsObjectHit` false)
  (set `self.GrappleObjectState` "NewEnumerator0"))

(fn `TickRetracted`
  (bind _owningcharacter (`self.OwningCharacter`))
  (`/Engine/EditorBlueprintResources/StandardMacros.IsValid` _owningcharacter
    (:`Is Valid`
      (bind _outactors (`KismetSystemLibrary.SphereOverlapActors` (`self.K2_GetActorLocation` _owningcharacter) (`self.MaxGrappleDistance`) (`|MakeArray` "ObjectTypeQuery1" :!type "EObjectTypeQuery Enum") "/Game/Blueprint/Pisto-outils/Attrapistolet/BP_AttrapistoletTarget.BP_AttrapistoletTarget_C"))
      (bind _target (`self.FindBestTarget` _outactors))
      (`self.SetCurrentTarget` (cast `/Game/Blueprint/Pisto-outils/Attrapistolet/BP_AttrapistoletTarget` _target :!pure true)))))

(fn `TickRetractedObject`)

(fn `TickVelocityLaunch`
  (bind _asprimitive_component (cast `PrimitiveComponent` (`Actor.RootComponent` (`self.GrappleObjectTarget`))))
  (bind _outlaunchvelocity (`GameplayStatics.SuggestProjectileVelocity_CustomArc` (`SceneComponent.K2_GetComponentLocation` _asprimitive_component) (`self.K2_GetActorLocation` (`GameplayStatics.GetPlayerCharacter` 0)) 0.0 0.8))
  (`PrimitiveComponent.AddImpulse` _asprimitive_component _outlaunchvelocity "None" true)
  (set `self.GrappleObjectState` "NewEnumerator4"))

(fn `UserConstructionScript`)