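; BP_AttrapistoletHook is the grappling hook projectile of the Attrapistolet, flying from its spawn point to a target.
; On BeginPlay it aims ProjectileMovement once at ObjectTarget or Target, depending on IsObjectHit.
; Tick compares squared distances from the start to detect arrival, then stops the hook, snaps it to EndingLocation (refreshed only for ObjectTarget) and plays GrappleEnd once.
; DistanceToTarget exposes the remaining distance.
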(event `self.ReceiveBeginPlay`
  (if (`self.isObjectHit`)
    (bind _objecttarget (`self.ObjectTarget`)
      (:`then`
        (set `self.StartingLocation` (`self.K2_GetActorLocation`))
        (set `self.EndingLocation` (`self.K2_GetActorLocation` _objecttarget)))
      (:`else`))
    (else
      (bind _target (`self.Target`)
        (:`then`
          (set `self.StartingLocation` (`self.K2_GetActorLocation`))
          (set `self.EndingLocation` (`self.K2_GetActorLocation` _target)))
        (:`else`))))
  (set `self.Direction` (`KismetMathLibrary.Normal` (- (`self.EndingLocation`) (`self.StartingLocation`))))
  (set `MovementComponent.Velocity` (* (`self.Direction`) (`self.Speed`)) (`self.ProjectileMovement`)))

(event `self.ReceiveTick`
  (params (DeltaSeconds :type "Float (single-precision)"))
  (bind _endinglocation (`self.EndingLocation`))
  (bind _startinglocation (`self.StartingLocation`))
  (bind _startinglocation_2 (`self.StartingLocation`))
  (if (`self.isObjectHit`)
    (bind _objecttarget (`self.ObjectTarget`)
      (:`then`
        (set `self.EndingLocation` (`SceneComponent.K2_GetComponentLocation` (`Actor.RootComponent` _objecttarget)))
        (if (>= (`KismetMathLibrary.Vector_DistanceSquared` (`self.K2_GetActorLocation`) _startinglocation_2) (`KismetMathLibrary.Vector_DistanceSquared` (`self.K2_GetActorLocation` _objecttarget) _startinglocation_2))
          (`self.K2_SetActorLocation` _endinglocation :!label _label)
          (set `MovementComponent.Velocity` (0.0 0.0 0.0) (`self.ProjectileMovement`))
          (`/Engine/EditorBlueprintResources/StandardMacros.DoOnce` false
            (:`Completed`
              (`GameplayStatics.PlaySoundAtLocation` "/Game/Blueprint/Pisto-outils/Attrapistolet/GrappleEnd.GrappleEnd" _endinglocation (struct) 1.0 1.0 0.0 null null null null)))))
      (:`else`))
    (else
      (bind _target (`self.Target`)
        (:`then`
          (if (>= (`KismetMathLibrary.Vector_DistanceSquared` (`self.K2_GetActorLocation`) _startinglocation) (`KismetMathLibrary.Vector_DistanceSquared` (`self.K2_GetActorLocation` _target) _startinglocation))
            (goto _label)))
        (:`else`)))))

(fn `DistanceToTarget`
  (returns (ReturnValue :type "Float (double-precision)"))
  (return (`KismetMathLibrary.Vector_Distance` (`self.EndingLocation`) (`self.K2_GetActorLocation`))))

(fn `UserConstructionScript`)