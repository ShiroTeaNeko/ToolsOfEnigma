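; Interactable story actor that shows a text message when the first-person player presses F nearby, then destroys itself.
; Overlapping Box enables input, creates the story widget with InteractionText and opens a Gate for the F key; leaving reverses input and gate.
; F displays the widget for a configurable duration before removal.
; A separate DetectCollision volume shows and hides the UIInteract prompt, which RemoveInteract can also clear.
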(event `Key|F`
  (params (Key :type "Key Structure"))
  (:`Pressed`
    (`/Engine/EditorBlueprintResources/StandardMacros.Gate` true :!label _label
      (:`Exit`
        (`UserWidget.AddToViewport` (stale `self.Box.OnComponentBeginOverlap` _returnvalue) 0)
        (`KismetSystemLibrary.Delay` (`self.Durée affichage text (sec)`))
        (`Widget.RemoveFromParent` (stale `self.Box.OnComponentBeginOverlap` _returnvalue))
        (`self.K2_DestroyActor`)))))

(event `self.Box.OnComponentBeginOverlap`
  (params (OverlappedComponent :type "PrimitiveComponent Object Reference") (OtherActor :type "Actor Object Reference") (OtherComp :type "PrimitiveComponent Object Reference") (OtherBodyIndex :type Integer) (bFromSweep :type Boolean) (SweepResult :type "HitResult Structure (by ref)"))
  (cast `/Game/FirstPerson/Blueprints/BP_FirstPersonCharacter` OtherActor)
  (`self.EnableInput` (`GameplayStatics.GetPlayerController` 0))
  (bind _returnvalue (`|CreateWidget` "/Game/Blueprint/BP_Story/Interact_Story_Widget.Interact_Story_Widget_C"))
  (set `/Game/Blueprint/BP_Story/Interact_Story_Widget.Interaction Text` (`self.Interaction Text`) _returnvalue)
  (goto _label :!via `Open`))

(event `self.Box.OnComponentEndOverlap`
  (params (OverlappedComponent :type "PrimitiveComponent Object Reference") (OtherActor :type "Actor Object Reference") (OtherComp :type "PrimitiveComponent Object Reference") (OtherBodyIndex :type Integer))
  (cast `/Game/FirstPerson/Blueprints/BP_FirstPersonCharacter` OtherActor)
  (`self.DisableInput` (`GameplayStatics.GetPlayerController` 0))
  (goto _label :!via `Close`))

(event `self.DetectCollision.OnComponentBeginOverlap`
  (params (OverlappedComponent :type "PrimitiveComponent Object Reference") (OtherActor :type "Actor Object Reference") (OtherComp :type "PrimitiveComponent Object Reference") (OtherBodyIndex :type Integer) (bFromSweep :type Boolean) (SweepResult :type "HitResult Structure (by ref)"))
  (cast `/Game/FirstPerson/Blueprints/BP_FirstPersonCharacter` OtherActor)
  (`/Engine/EditorBlueprintResources/StandardMacros.IsValid` (`self.UIInteract`)
    (:`Is Not Valid`
      (bind _returnvalue (`|CreateWidget` "/Game/Alexis/UI/UIInteract.UIInteract_C"))
      (bind _output_get (set `self.UIInteract` _returnvalue))
      (`UserWidget.AddToViewport` _output_get 0))))

(event `self.DetectCollision.OnComponentEndOverlap`
  (params (OverlappedComponent :type "PrimitiveComponent Object Reference") (OtherActor :type "Actor Object Reference") (OtherComp :type "PrimitiveComponent Object Reference") (OtherBodyIndex :type Integer))
  (cast `/Game/FirstPerson/Blueprints/BP_FirstPersonCharacter` OtherActor)
  (`/Engine/EditorBlueprintResources/StandardMacros.IsValid` (`self.UIInteract`) :!label _label_2
    (:`Is Valid`
      (`Widget.RemoveFromParent` (`self.UIInteract`))
      (set `self.UIInteract` null))))

(event `RemoveInteract`
  (goto _label_2))

(fn `UserConstructionScript`)