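; BP_BoardPlace is a puzzle board that tracks whether all of its child pieces are correct.
; BlockFinish starts with collision disabled on BeginPlay.
; CheckIfBoardFinish, which has no caller in this Blueprint, scans AllChild through GetIsCorrect and stops at the first incorrect piece.
; When all are correct it switches BlockFinish to query-only collision, and either outcome prints a debug message, with success labelled as the blue puzzle.
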(event `self.ReceiveBeginPlay`
  (`PrimitiveComponent.SetCollisionEnabled` (`self.BlockFinish`) "NoCollision"))

(fn `CheckIfBoardFinish`
  (set `self.IsPuzzleFinish` true)
  (for _array_element (`self.AllChild`)
    (bind _iscorrect (`/Game/Alexis/BP/BP_BoardPlaceSlot.GetIsCorrect` _array_element))
    (if (not _iscorrect)
      (set `self.IsPuzzleFinish` false)
      (break)))
  (if (`self.IsPuzzleFinish`)
    (`KismetSystemLibrary.PrintString` "PUZLLE BLUE FINISH" true true (struct :`G` 0.139282 :`B` 1.0 :`A` 1.0))
    (`PrimitiveComponent.SetCollisionEnabled` (`self.BlockFinish`) "QueryOnly")
    (else
      (`KismetSystemLibrary.PrintString` "NOT FINISH"))))

(fn `UserConstructionScript`)