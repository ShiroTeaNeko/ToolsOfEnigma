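; BP_DoorDropPipe is a puzzle-driven door that opens once enough enigmas are finished.
; Each EnigmaFinish event increments a counter and compares it to AmountToFinish.
; When the threshold is met, MoveComponentTo swings the PivotWL and PivotWR pivots in opposite directions with an eased one-second rotation.
; The counter never resets, so further events past the threshold reissue the same moves.
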(event `/Game/Alexis/BP/I_Enigma.EnigmaFinish`
  (bind _pivotwl (`self.PivotWL`))
  (bind _pivotwr (`self.PivotWR`))
  (bind _result (`/Engine/EditorBlueprintResources/StandardMacros.IncrementInt` (`self.CountEnigmaFinish`))
    (:`  `
      (if (>= _result (`self.AmountToFinish`))
        (`|ExecutionSequence`
          (:`then_0`
            (`KismetSystemLibrary.MoveComponentTo` _pivotwl (`SceneComponent.RelativeLocation` _pivotwl) (struct :`Yaw` -104.0) true false 1.0))
          (:`then_1`
            (`KismetSystemLibrary.MoveComponentTo` _pivotwr (`SceneComponent.RelativeLocation` _pivotwr) (struct :`Yaw` 125.0) true false 1.0)))))))

(fn `UserConstructionScript`)