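; BP_BoardRotate is an interactable puzzle board that manages a set of pipes and checks whether all are correct.
; Interact toggles between first person and the board camera with a short view blend, switching player movement and the mouse cursor.
; Leaving the board resets every pipe.
; CheckIfBoardFinish tests each pipe and, when all are correct, changes BlockFinish's collision and prints a debug message.
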(event `self.ReceiveBeginPlay`
  (`ActorComponent.SetActive` (`self.Camera`) false false))

(event `self.ReceiveTick`
  (params (DeltaSeconds :type "Float (single-precision)")))

(fn `CheckIfBoardFinish`
  (set `self.IsPuzzleFinish` true)
  (for _array_element (`self.AllPipe`)
    (bind _iscorrect (`/Game/Alexis/BP/BP_BoardRotateSlot.GetIsCorrect` _array_element))
    (if (not _iscorrect)
      (set `self.IsPuzzleFinish` false)
      (break)))
  (if (`self.IsPuzzleFinish`)
    (`KismetSystemLibrary.PrintString` "PUZLLE BLUE FINISH" true true (struct :`G` 0.139282 :`B` 1.0 :`A` 1.0))
    (`PrimitiveComponent.SetCollisionEnabled` (`self.BlockFinish`) "QueryOnly")
    (`PrimitiveComponent.SetCollisionProfileName` (`self.BlockFinish`) "BlockAllDynamic" true)
    (else
      (`KismetSystemLibrary.PrintString` "NOT FINISH"))))

(fn `Interact`
  (params (Player :type "/Game/FirstPerson/Blueprints/BP_FirstPersonCharacter Object Reference"))
  (returns (bIsSucess :type Boolean))
  (bind _isfpsactive (`/Game/FirstPerson/Blueprints/BP_FirstPersonCharacter.IsFPSActive` Player))
  (`ActorComponent.SetActive` (`self.Camera`) _isfpsactive false)
  (if _isfpsactive
    (set `self.PuzzleActiv?` true)
    (set `/Game/FirstPerson/Blueprints/BP_FirstPersonCharacter.IsFPSActive` false Player)
    (`PlayerController.SetViewTargetWithBlend` (`GameplayStatics.GetPlayerController` 0) (`ActorComponent.GetOwner` (`self.Camera`)) 0.2 "VTBlend_Linear" 0.0 true)
    (set `/Game/FirstPerson/Blueprints/BP_FirstPersonCharacter.CanMove` false Player)
    (set `PlayerController.bShowMouseCursor` true (`GameplayStatics.GetPlayerController` 0))
    (return true)
    (else
      (set `self.PuzzleActiv?` false)
      (set `/Game/FirstPerson/Blueprints/BP_FirstPersonCharacter.IsFPSActive` true Player)
      (`PlayerController.SetViewTargetWithBlend` (`GameplayStatics.GetPlayerController` 0) (`ActorComponent.GetOwner` (`/Game/FirstPerson/Blueprints/BP_FirstPersonCharacter.FirstPersonCamera` Player)) 0.2 "VTBlend_Linear" 0.0 true)
      (set `/Game/FirstPerson/Blueprints/BP_FirstPersonCharacter.CanMove` true Player)
      (set `PlayerController.bShowMouseCursor` false (`GameplayStatics.GetPlayerController` 0))
      (`self.ResetAllPipePos`)
      (return true))))

(fn `ResetAllPipePos`
  (for _array_element (`self.AllPipe`)
    (`/Game/Alexis/BP/BP_BoardRotateSlot.ResetPos` _array_element)))

(fn `UserConstructionScript`)