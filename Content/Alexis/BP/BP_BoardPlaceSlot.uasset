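; BP_BoardPlaceSlot is one slot on a pipe puzzle board that holds a single pipe and tracks whether it is the correct one.
; PlacePipe snaps a pipe to the Sphere's PipeHolder socket if empty, rotates it, checks correctness and notifies BoardRef.
; Correctness requires matching CorrectPipe class and CorrectRotation.
; GetIsCorrect reports false for empty slots, using the Sphere's child count as occupancy.
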(event `self.ReceiveTick`
  (params (DeltaSeconds :type "Float (single-precision)")))

(fn `CheckIfCorrect`
  (set `self.IsCorrectPipe` false)
  (if (== (`GameplayStatics.GetObjectClass` (`self.Pipe`)) (`self.CorrectPipe`))
    (if (`|EnumEquality` (`/Game/Alexis/BP/BP_Pipe.Rotation` (`self.Pipe`)) (`self.CorrectRotation`))
      (set `self.IsCorrectPipe` true))))

(fn `GetIsCorrect`
  (returns (IsCorrect :type Boolean))
  (if (not (> (`SceneComponent.GetNumChildrenComponents` (`self.Sphere`)) 0))
    (set `self.IsCorrectPipe` false))
  (return (`self.IsCorrectPipe`)))

(fn `PlacePipe`
  (params (Pipe :type "/Game/Alexis/BP/BP_Pipe Object Reference"))
  (bind _boardref (`self.BoardRef`))
  (if (> (`SceneComponent.GetNumChildrenComponents` (`self.Sphere`)) 0)
    (`KismetSystemLibrary.PrintString` "Hello")
    (else
      (`KismetSystemLibrary.PrintString` "HFSDFSDFSDello")
      (bind _output_get (set `self.Pipe` Pipe))
      (`self.K2_AttachToComponent` _output_get (`self.Sphere`) "PipeHolder" "SnapToTarget" "SnapToTarget" "KeepWorld" true)
      (`/Game/Alexis/BP/BP_Pipe.RotatePipe` (`self.Pipe`))
      (`self.CheckIfCorrect`)
      (`/Engine/EditorBlueprintResources/StandardMacros.IsValid` _boardref
        (:`Is Valid`
          (`/Game/Alexis/BP/BP_BoardPlace.CheckIfBoardFinish` _boardref))))))

(fn `UserConstructionScript`)