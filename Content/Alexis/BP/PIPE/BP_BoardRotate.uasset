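; Pipe puzzle board that the first-person player uses through a fixed camera, with an interact prompt shown inside its overlap zone.
; Interact toggles between player and board views, switching movement, visibility and mouse cursor, and calls ResetPos on every pipe when leaving.
; CheckIfBoardFinish tests all pipes; when all are correct, it notifies an I_Enigma actor, enables the BlockFinish collision, exits via Interact and plays a sound.
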(event `self.ReceiveBeginPlay`
  (`ActorComponent.SetActive` (`self.Camera`) false false))

(event `self.ReceiveTick`
  (params (DeltaSeconds :type "Float (single-precision)")))

(event `self.DetectCollision.OnComponentBeginOverlap`
  (params (OverlappedComponent :type "PrimitiveComponent Object Reference") (OtherActor :type "Actor Object Reference") (OtherComp :type "PrimitiveComponent Object Reference") (OtherBodyIndex :type Integer) (bFromSweep :type Boolean) (SweepResult :type "HitResult Structure (by ref)"))
  (cast `/Game/FirstPerson/Blueprints/BP_FirstPersonCharacter` OtherActor)
  (`/Engine/EditorBlueprintResources/StandardMacros.IsValid` (`self.UIInteract`)
    (:`Is Not Valid`
      (bind _returnvalue (`|CreateWidget` "/Game/Alexis/UI/UIInteract.UIInteract_C"))
      (bind _output_get (set `self.UIInteract` _returnvalue))
      (`UserWidget.AddToViewport` _returnvalue 0)
      (`UserWidget.AddToViewport` _output_get 0))))

(event `self.DetectCollision.OnComponentEndOverlap`
  (params (OverlappedComponent :type "PrimitiveComponent Object Reference") (OtherActor :type "Actor Object Reference") (OtherComp :type "PrimitiveComponent Object Reference") (OtherBodyIndex :type Integer))
  (cast `/Game/FirstPerson/Blueprints/BP_FirstPersonCharacter` OtherActor)
  (`/Engine/EditorBlueprintResources/StandardMacros.IsValid` (`self.UIInteract`) :!label _label
    (:`Is Valid`
      (`Widget.RemoveFromParent` (`self.UIInteract`))
      (set `self.UIInteract` null))))

(event `RemoveInteract`
  (goto _label))

(fn `CheckIfBoardFinish`
  (set `self.IsPuzzleFinish` true)
  (for _array_element (`self.AllPipe`)
    (bind _iscorrect (`/Game/Alexis/BP/PIPE/BP_BoardRotateSlot.GetIsCorrect` _array_element))
    (if (not _iscorrect)
      (set `self.IsPuzzleFinish` false)
      (break)))
  (if (`self.IsPuzzleFinish`)
    (if (`KismetSystemLibrary.DoesImplementInterface` (`self.ActorEnigmaComplete`) "/Game/Alexis/BP/I_Enigma.I_Enigma_C")
      (message `/Game/Alexis/BP/I_Enigma.EnigmaFinish` (`self.ActorEnigmaComplete`))
      (`PrimitiveComponent.SetCollisionEnabled` (`self.BlockFinish`) "QueryOnly")
      (`PrimitiveComponent.SetCollisionProfileName` (`self.BlockFinish`) "BlockAllDynamic" true)
      (`self.Interact` (`self.Player`))
      (`GameplayStatics.PlaySoundAtLocation` "/Game/Sound/Achievement-Sound-Effect.Achievement-Sound-Effect" (0.0 0.0 0.0) (struct) 1.0 1.0 0.0 null null null null))))

(fn `Interact`
  (params (Player :type "/Game/FirstPerson/Blueprints/BP_FirstPersonCharacter Object Reference"))
  (returns (bIsSucess :type Boolean))
  (bind _output_get (set `self.Player` Player))
  (bind _isfpsactive (`/Game/FirstPerson/Blueprints/BP_FirstPersonCharacter.IsFPSActive` _output_get))
  (`ActorComponent.SetActive` (`self.Camera`) _isfpsactive false)
  (if _isfpsactive
    (set `self.PuzzleActiv?` true)
    (set `/Game/FirstPerson/Blueprints/BP_FirstPersonCharacter.IsFPSActive` false (`self.Player`))
    (`self.SetActorHiddenInGame` (`self.Player`) true)
    (`PlayerController.SetViewTargetWithBlend` (`GameplayStatics.GetPlayerController` 0) (`ActorComponent.GetOwner` (`self.Camera`)) 0.2 "VTBlend_Linear" 0.0 true)
    (set `/Game/FirstPerson/Blueprints/BP_FirstPersonCharacter.CanMove` false (`self.Player`))
    (set `PlayerController.bShowMouseCursor` true (`GameplayStatics.GetPlayerController` 0))
    (`self.RemoveInteract`)
    (return true)
    (else
      (set `self.PuzzleActiv?` false)
      (set `/Game/FirstPerson/Blueprints/BP_FirstPersonCharacter.IsFPSActive` true (`self.Player`))
      (`PlayerController.SetViewTargetWithBlend` (`GameplayStatics.GetPlayerController` 0) (`ActorComponent.GetOwner` (`/Game/FirstPerson/Blueprints/BP_FirstPersonCharacter.FirstPersonCamera` (`self.Player`))) 0.2 "VTBlend_Linear" 0.0 true)
      (`self.SetActorHiddenInGame` (`self.Player`) false)
      (set `/Game/FirstPerson/Blueprints/BP_FirstPersonCharacter.CanMove` true (`self.Player`))
      (set `PlayerController.bShowMouseCursor` false (`GameplayStatics.GetPlayerController` 0))
      (`self.ResetAllPipePos`)
      (return true))))

(fn `ResetAllPipePos`
  (for _array_element (`self.AllPipe`)
    (`/Game/Alexis/BP/PIPE/BP_BoardRotateSlot.ResetPos` _array_element)))

(fn `UserConstructionScript`)