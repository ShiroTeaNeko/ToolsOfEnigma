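; BP_BoardPlace is the board of a puzzle, in the PIPE folder, that detects when all its pieces are correct.
; BlockFinish starts with collision disabled.
; CheckIfBoardFinish polls each piece in AllChild, stopping at the first incorrect one and printing its name for debugging.
; When all are correct, it switches BlockFinish to query-only collision and calls EnigmaFinish on EventFinish.
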(event `self.ReceiveBeginPlay`
  (`PrimitiveComponent.SetCollisionEnabled` (`self.BlockFinish`) "NoCollision"))

(fn `CheckIfBoardFinish`
  (set `self.IsPuzzleFinish` true)
  (for _array_element (`self.AllChild`)
    (bind _iscorrect (`/Game/Alexis/BP/PIPE/BP_BoardPlaceSlot.GetIsCorrect` _array_element))
    (if (not _iscorrect)
      (`KismetSystemLibrary.PrintString` (`KismetSystemLibrary.GetDisplayName` _array_element))
      (set `self.IsPuzzleFinish` false)
      (break)))
  (if (`self.IsPuzzleFinish`)
    (`PrimitiveComponent.SetCollisionEnabled` (`self.BlockFinish`) "QueryOnly")
    (`/Game/Alexis/BP/I_Enigma.EnigmaFinish` (`self.EventFinish`))))

(fn `UserConstructionScript`)