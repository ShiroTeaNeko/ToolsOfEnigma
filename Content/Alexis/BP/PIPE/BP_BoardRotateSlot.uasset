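; BP_BoardRotateSlot is a clickable rotating tile in a board puzzle, apparently a pipe puzzle.
; While the board's puzzle is active, hovering makes the tile glow and clicking resets the board's pipe positions, then lifts, rolls and reseats it 90 degrees further using chained component moves.
; It then asks the board to check completion, with GetIsCorrect comparing rotation against accepted values.
; Interact calls forward to the board.
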(event `self.Box.OnClicked`
  (params (TouchedComponent :type "PrimitiveComponent Object Reference") (ButtonPressed :type "Key Structure"))
  (bind _box (`self.Box`))
  (bind _box_2 (`self.Box`))
  (bind _box_3 (`self.Box`))
  (bind _boardref (`self.BoardRef`))
  (bind (_relativelocation_x _relativelocation_y _relativelocation_z) (`KismetMathLibrary.BreakVector` (`SceneComponent.RelativeLocation` _box_3)))
  (bind (_relativelocation_x_2 _relativelocation_y_2 _relativelocation_z_2) (`KismetMathLibrary.BreakVector` (`SceneComponent.RelativeLocation` _box_2)))
  (bind (_relativerotation_roll _relativerotation_pitch _relativerotation_yaw) (`KismetMathLibrary.BreakRotator` (`SceneComponent.RelativeRotation` _box)))
  (if (`/Game/Alexis/BP/PIPE/BP_BoardRotate.PuzzleActiv?` _boardref) :!label _label
    (if (not (`self.IsRotating`))
      (set `self.IsRotating` true)
      (`/Game/Alexis/BP/PIPE/BP_BoardRotate.ResetAllPipePos` _boardref)
      (switch `/Game/Alexis/BP/E_Rotation` (`self.Rotation`)
        (:`NewEnumerator0`
          (set `self.Rotation` "NewEnumerator1"))
        (:`NewEnumerator1`
          (set `self.Rotation` "NewEnumerator2"))
        (:`NewEnumerator2`
          (set `self.Rotation` "NewEnumerator3"))
        (:`NewEnumerator3`
          (set `self.Rotation` "NewEnumerator0")))
      (`KismetSystemLibrary.MoveComponentTo` _box_2 (`KismetMathLibrary.MakeVector` _relativelocation_x_2 -30.0 _relativelocation_z_2) (`SceneComponent.RelativeRotation` _box_2) true)
      (`KismetSystemLibrary.MoveComponentTo` _box (`SceneComponent.RelativeLocation` _box) (`KismetMathLibrary.MakeRotator` (+ _relativerotation_roll 90.0) _relativerotation_pitch _relativerotation_yaw))
      (`KismetSystemLibrary.MoveComponentTo` _box_3 (`KismetMathLibrary.MakeVector` _relativelocation_x -2.0 _relativelocation_z) (`SceneComponent.RelativeRotation` _box_3) false true)
      (set `self.IsRotating` false)
      (`/Game/Alexis/BP/PIPE/BP_BoardRotate.CheckIfBoardFinish` _boardref)
      (set `self.IsActive` true))))

(event `self.Cube.OnClicked`
  (params (TouchedComponent :type "PrimitiveComponent Object Reference") (ButtonPressed :type "Key Structure"))
  (goto _label))

(event `self.Cube.OnEndCursorOver`
  (params (TouchedComponent :type "PrimitiveComponent Object Reference"))
  (`MeshComponent.SetScalarParameterValueOnMaterials` (`self.Cube`) "EmisiveMultiplier" 0.0 :!label _label_2)
  (set `self.IsActive` false))

(event `ResetPos`
  (set `self.IsActive` false))

(event `self.Box.OnEndCursorOver`
  (params (TouchedComponent :type "PrimitiveComponent Object Reference"))
  (goto _label_2))

(event `self.Box.OnBeginCursorOver`
  (params (TouchedComponent :type "PrimitiveComponent Object Reference"))
  (if (`/Game/Alexis/BP/PIPE/BP_BoardRotate.PuzzleActiv?` (`self.BoardRef`)) :!label _label_3
    (if (not (`self.IsActive`))
      (`MeshComponent.SetScalarParameterValueOnMaterials` (`self.Cube`) "EmisiveMultiplier" 10.0))))

(event `self.Cube.OnBeginCursorOver`
  (params (TouchedComponent :type "PrimitiveComponent Object Reference"))
  (goto _label_3))

(fn `GetIsCorrect`
  (returns (IsCorrect :type Boolean))
  (locals (IsCorrectRot :type Boolean))
  (for _array_element (`self.CorrectRot`)
    (if (`|EnumEquality` _array_element (`self.Rotation`))
      (set `local.IsCorrectRot` true)
      (break)))
  (return (`local.IsCorrectRot`)))

(fn `Interact`
  (params (Player :type "/Game/FirstPerson/Blueprints/BP_FirstPersonCharacter Object Reference"))
  (returns (bIsSucess :type Boolean))
  (`/Game/Alexis/BP/I_Interact.Interact` (`self.BoardRef`) Player)
  (return false))

(fn `UserConstructionScript`)