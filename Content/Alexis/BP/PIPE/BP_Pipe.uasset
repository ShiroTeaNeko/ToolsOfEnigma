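; BP_Pipe is a pipe puzzle piece that the first-person player picks up and drops onto board slots.
; Pickup rolls its Box by an angle taken from Rotation; dropping line-traces from the player camera and passes the pipe to any BP_BoardPlaceSlot hit.
; When not held, it returns to its start position if it strays too far, checked on drop and through a delayed Tick.
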(event `self.ReceiveBeginPlay`
  (set `self.StartPosition` (`self.K2_GetActorLocation`))
  (bind _asbp_first_person_character (cast `/Game/FirstPerson/Blueprints/BP_FirstPersonCharacter` (`GameplayStatics.GetPlayerCharacter` 0)))
  (set `self.FPS` _asbp_first_person_character))

(event `self.ReceiveTick`
  (params (DeltaSeconds :type "Float (single-precision)"))
  (if (not (`self.IsPick?`))
    (`KismetSystemLibrary.Delay` 3.0)
    (if (`self.IsPick?`)
      _
      (elif (> (`KismetMathLibrary.Vector_Distance` (`self.StartPosition`) (`self.K2_GetActorLocation`)) 500.0)
        (`self.K2_SetActorLocation` (`self.StartPosition`))))))

(event `/Game/Alexis/BP/I_Pickupable.OnPickup`
  (set `self.IsPick?` true)
  (`self.RotatePipe`))

(event `/Game/Alexis/BP/I_Pickupable.OnDrop`
  (bind _firstpersoncamera (`/Game/FirstPerson/Blueprints/BP_FirstPersonCharacter.FirstPersonCamera` (`self.FPS`)))
  (bind _returnvalue (`SceneComponent.K2_GetComponentLocation` _firstpersoncamera))
  (set `self.IsPick?` false)
  (if (> (`KismetMathLibrary.Vector_Distance` (`self.StartPosition`) (`self.K2_GetActorLocation`)) 500.0)
    (`self.K2_SetActorLocation` (`self.StartPosition`)))
  (bind _outhit (`KismetSystemLibrary.LineTraceSingle` :`Start` _returnvalue :`End` (+ _returnvalue (* (`SceneComponent.GetForwardVector` _firstpersoncamera) 2000.0)) :`TraceChannel` "TraceTypeQuery1" :`DrawDebugType` "ForDuration" :`DrawTime` 1.5))
  (bind (_bblockinghit _binitialoverlap _time _distance _location _impactpoint _normal _impactnormal _physmat _hitactor) (`GameplayStatics.BreakHitResult` _outhit))
  (bind _asbp_board_place_slot (cast `/Game/Alexis/BP/PIPE/BP_BoardPlaceSlot` _hitactor)
    (:`then`
      (`/Game/Alexis/BP/PIPE/BP_BoardPlaceSlot.PlacePipe` _asbp_board_place_slot self))
    (:`CastFailed`
      (`KismetSystemLibrary.PrintString` "Cast Failed")
      (`KismetSystemLibrary.PrintString` (`KismetSystemLibrary.GetDisplayName` _hitactor)))))

(fn `RotatePipe`
  (switch `/Game/Alexis/BP/E_Rotation` (`self.Rotation`)
    (:`NewEnumerator0`
      (set `self.Int` 0))
    (:`NewEnumerator1`
      (set `self.Int` 90))
    (:`NewEnumerator2`
      (set `self.Int` 180))
    (:`NewEnumerator3`
      (set `self.Int` 270)))
  (`SceneComponent.K2_AddLocalRotation` (`self.Box`) (`KismetMathLibrary.MakeRotator` (`KismetMathLibrary.Conv_IntToDouble` (`self.Int`))) false false))

(fn `UserConstructionScript`)