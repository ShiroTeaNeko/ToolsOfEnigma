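; BP_BoardRotateSlot is a clickable slot for a board that appears to be a pipe puzzle.
; Clicking its cube calls the board's ResetAllPipePos and then marks the slot active, while ResetPos clears that state.
; Hovering an inactive slot raises an emissive material parameter as a highlight, cleared when the cursor leaves.
; Interact forwards the player to the board reference and returns false.
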(event `self.Cube.OnClicked`
  (params (TouchedComponent :type "PrimitiveComponent Object Reference") (ButtonPressed :type "Key Structure"))
  (`/Game/Alexis/BP/BP_BoardRotate.ResetAllPipePos` (`self.BoardRef`))
  (set `self.IsActive` true))

(event `self.Cube.OnEndCursorOver`
  (params (TouchedComponent :type "PrimitiveComponent Object Reference"))
  (`MeshComponent.SetScalarParameterValueOnMaterials` (`self.Cube`) "EmisiveMultiplier" 0.0))

(event `ResetPos`
  (set `self.IsActive` false))

(event `self.Cube.OnBeginCursorOver`
  (params (TouchedComponent :type "PrimitiveComponent Object Reference"))
  (if (not (`self.IsActive`))
    (`MeshComponent.SetScalarParameterValueOnMaterials` (`self.Cube`) "EmisiveMultiplier" 10.0)))

(fn `Interact`
  (params (Player :type "/Game/FirstPerson/Blueprints/BP_FirstPersonCharacter Object Reference"))
  (returns (bIsSucess :type Boolean))
  (`/Game/Alexis/BP/I_Interact.Interact` (`self.BoardRef`) Player)
  (return false))

(fn `UserConstructionScript`)